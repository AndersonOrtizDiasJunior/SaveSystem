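; BP_SaveGameActor is a placeable save point that lets the player open the save UI when nearby.
; Sphere overlap with the player toggles a WBP_SaveAction prompt widget, the CanSave flag and actor input.
; Pressing a key in TriggerKeys opens the saving component's UI in save mode.
; With UseOwnCamera, it first assigns its child-actor BP_SaveLoadManager as that component's TemporaryCamera for the thumbnail.
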(event OnComponentBeginOverlap(Sphere)
  (params (OverlappedComponent :type Primitive%20Component%20Object%20Reference) (OtherActor :type Actor%20Object%20Reference) (OtherComp :type Primitive%20Component%20Object%20Reference) (OtherBodyIndex :type Integer) (bFromSweep :type Boolean) (SweepResult :type Hit%20Result%20Structure%20%28by%20ref%29))
  ;[1 1 1] Overlap Events
  (if (== OtherActor (Game|GetPlayerCharacter 0))
    (Rendering|SetVisibility (Variables|Default|GetWidget) true false)
    (Variables|Default|SetbCanSave true)
    (Input|EnableInput (Game|GetPlayerController 0))))

(event OnComponentEndOverlap(Sphere)
  (params (OverlappedComponent :type Primitive%20Component%20Object%20Reference) (OtherActor :type Actor%20Object%20Reference) (OtherComp :type Primitive%20Component%20Object%20Reference) (OtherBodyIndex :type Integer))
  ;[1 1 1] Overlap Events
  (if (== OtherActor (Game|GetPlayerCharacter 0))
    (Rendering|SetVisibility (Variables|Default|GetWidget) false false)
    (Variables|Default|SetbCanSave false)
    (Input|DisableInput self (Game|GetPlayerController 0))))

(event EventBeginPlay
  ;[1 1 1] Setup
  (bind _returnvalue (UserInterface|CreateWidget "/CompleteSaveSystem/Widgets/Misc/WBP_SaveAction.WBP_SaveAction_C" 0 (Variables|Default|GetInput%20Action%20Row)))
  (UserInterface|SetWidget (Variables|Default|GetWidget) _returnvalue))

(event Input|KeyboardEvents|AnyKey
  (params (Key :type Key%20Structure :default "None"))
  ;[1 1 1] Input Handling
  (:Pressed
    (if (and (Utilities|Array|ContainsItem (Variables|Default|GetTriggerKeys) Key) (Variables|Default|GetbCanSave))
      (if (Variables|Default|GetbUseOwnCamera)
        (|UpdateThumbnail))
      (Default|OpenUI (CallFunction|GetSavingComponent) false))))

(fn ConstructionScript)