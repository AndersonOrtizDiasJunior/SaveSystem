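; BP_Checkpoint is a placeable auto-save checkpoint that fires when the player character overlaps its collision.
; A ShouldSave check passes only if the saving component has finished loading and this checkpoint's name is not already saved.
; It then shows the WBP_AutoSave widget, records the checkpoint name and writes an auto save to the next slot index.
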(event OnComponentBeginOverlap(Collision)
  (params (OverlappedComponent :type Primitive%20Component%20Object%20Reference) (OtherActor :type Actor%20Object%20Reference) (OtherComp :type Primitive%20Component%20Object%20Reference) (OtherBodyIndex :type Integer) (bFromSweep :type Boolean) (SweepResult :type Hit%20Result%20Structure%20%28by%20ref%29))
  (if (== OtherActor (Game|GetPlayerCharacter 0))
    (Utilities|ShouldSave?
      (:Yes
        (CallFunction|CallWidget)
        (CallFunction|SaveGame)))))

(event Custom|CallWidget
  (bind _returnvalue (UserInterface|CreateWidget "/CompleteSaveSystem/Widgets/Misc/WBP_AutoSave.WBP_AutoSave_C"))
  (UserInterface|Viewport|AddtoViewport _returnvalue 0))

(event Custom|SaveGame
  (bind _component (CallFunction|GetSavingComponent))
  (Default|AddSavedCheckpoint (CallFunction|GetSavingComponent) (Variables|Default|GetCheckpointName))
  (Default|SaveGame _component (Default|GetNextSlotIndex _component) true))

(fn ConstructionScript)