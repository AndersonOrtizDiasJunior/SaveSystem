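; Save/load manager Blueprint that captures save thumbnails and relays the saving component's load-finished event.
; On BeginPlay it can snap-attach to the player's camera component.
; GetThumbnail renders a scene capture, chosen via GetCameraToUse with an optional temporary camera, into a new render target.
; The target converts asynchronously to a texture, whose save data goes to BP_SavingComponent to finish the thumbnail.
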(event OnFinishLoading(BP_SavingComponent)
  (Default|CallOnFinishLoading))

(event Custom|GetThumbnail
  (params (TemporaryCamera :type Scene%20Capture%20Component%202D%20Object%20Reference))
  (bind _camtouse (|GetCameratoUse TemporaryCamera))
  (bind _returnvalue (Rendering|CreateRenderTarget2D 1024 1024 "RTF_RGBA8"))
  (Variables|/Script/Engine.SceneCaptureComponent2D|SetTextureTarget _camtouse _returnvalue)
  (Rendering|SceneCapture|CaptureScene _camtouse :!class /Script/Engine.SceneCaptureComponent2D)
  (Class|TextureSavingFunctionLibrary|RenderTargettoTexture2DAsync _returnvalue (delegate Custom|OnFinishConverting)))

(event Custom|OnFinishConverting
  (params (NewTexture :type Texture%202D%20Object%20Reference))
  (bind _returnvalue (Class|TextureSavingFunctionLibrary|GetTextureSaveData NewTexture))
  (Default|FinishThumbnail (Variables|Default|GetBP_SavingComponent) _returnvalue))

(event EventBeginPlay
  (if (Variables|Default|GetAttachToPlayerCamera)
    (bind _output_get (Variables|Default|SetPlayerCamera (Actor|GetComponentbyClass (Game|GetPlayerCharacter 0) "/Script/Engine.CameraComponent")))
    (Transformation|AttachComponentToComponent _output_get "None" "SnapToTarget" "SnapToTarget" "SnapToTarget" true)))

(fn ConstructionScript)