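; BP_ThumbnailCamera is a scene capture actor that produces thumbnail data from the game view.
; On BeginPlay it optionally snaps itself onto the player character's camera component so captures match the player's view.
; GetThumbnail creates a fresh 1024-square render target on each call, captures the scene into it and returns it converted to save data, printing a message on failure.
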(event EventBeginPlay
  (if (Variables|Default|GetAttachToPlayerCamera)
    (bind _output_get (Variables|Default|SetPlayerCamera (Actor|GetComponentbyClass (Game|GetPlayerCharacter 0) "/Script/Engine.CameraComponent")))
    (Transformation|AttachComponentToComponent _output_get "None" "SnapToTarget" "SnapToTarget" "SnapToTarget" true)))

(fn ConstructionScript)

(fn GetThumbnail
  (bind _scenecapturecomponent2d (Variables|Default|GetSceneCaptureComponent2D))
  (bind _returnvalue (Rendering|CreateRenderTarget2D 1024 1024 "RTF_RGBA8"))
  (Variables|/Script/Engine.SceneCaptureComponent2D|SetTextureTarget _scenecapturecomponent2d _returnvalue)
  (Rendering|SceneCapture|CaptureScene _scenecapturecomponent2d :!class /Script/Engine.SceneCaptureComponent2D)
  (bind _savedata (Utilities|GetRenderTargetSaveData _returnvalue)
    (:Succes
      (return _savedata))
    (:Failure
      (Development|PrintString "Failure"))))